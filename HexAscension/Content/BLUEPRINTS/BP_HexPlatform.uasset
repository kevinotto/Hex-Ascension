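; Hexagonal platform actor that changes its height by scaling the ScalingTile component along Z.
; SetPlatformHeight adds the given amount to CurrentHeight as the new target and plays the EnableHeightChange timeline, which flags the change as active.
; While flagged, Tick sets a clamped Z scale using FInterpTo from the stored CurrentHeight, which only updates to the target when the timeline finishes.
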(event `self.ReceiveTick`
  (params (DeltaSeconds :type "Float (single-precision)"))
  (bind (_returnvalue_x _returnvalue_y) (`KismetMathLibrary.BreakVector` (`SceneComponent.K2_GetComponentScale` (`self.ScalingTile`))))
  (if (`self.ChangingHeight`)
    (`SceneComponent.SetWorldScale3D` (`self.ScalingTile`) (`KismetMathLibrary.MakeVector` _returnvalue_x _returnvalue_y (`KismetMathLibrary.FClamp` (`KismetMathLibrary.FInterpTo` (`self.CurrentHeight`) (`self.NextHeight`) (`GameplayStatics.GetWorldDeltaSeconds`) 6.0) 1.32 2000.0)))))

(event `/Game/BLUEPRINTS/BPI_Interface.SetPlatformHeight`
  (params (NewHeight :type "Float (double-precision)"))
  ;[1 0.4688 0.4688] Set Platform Height
  (set `self.NextHeight` (+ NewHeight (`self.CurrentHeight`)))
  (`Timeline|EnableHeightChange` :!via `PlayFromStart`
    (:`Update`
      (set `self.ChangingHeight` true))
    (:`Finished`
      (set `self.ChangingHeight` false)
      (set `self.CurrentHeight` (`self.NextHeight`)))))

(event `self.ReceiveBeginPlay`)

(fn `UserConstructionScript`)