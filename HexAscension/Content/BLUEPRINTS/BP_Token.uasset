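; Token actor representing a random data storage medium, from scroll to SSD, that changes a platform's height when dropped or picked up.
; BeginPlay picks one of eight types, setting its mesh and height value, and starts a timeline bob.
; TokenDrop sphere-traces down for a "Platform"-tagged actor, messages it the value and enables box collision.
; TokenPickup sends the negated value to the stored platform and disables that collision.
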(event `self.ReceiveBeginPlay`
  (`|ExecutionSequence`
    (:`then_0`
      ;[0.06864 0.07497 0.25] Bobbin
      (bind (_direction _bobbin) (`Timeline|ItemBob`)
        (:`Update`
          (`SceneComponent.K2_SetRelativeLocation` (`self.FollowEmpty`) (`KismetMathLibrary.MakeVector` 0.0 0.0 _bobbin) false false))))
    (:`then_1`
      ;[0.1531 0.1927 0.02809] Set token randomly
      (set `self.TokenMeshList` (cast `/Game/BLUEPRINTS/TokenMeshList` (`KismetMathLibrary.Conv_IntToByte` (`KismetMathLibrary.RandomIntegerInRange` 0 7)))))
    (:`then_2`
      ;[0.04383 0.2031 0.01688] Set static mesh and give token its value
      (switch `/Game/BLUEPRINTS/TokenMeshList` (`self.TokenMeshList`)
        (:`NewEnumerator0`
          (set `self.SetMesh` "/Game/ASSETS/UMJ2023_Scroll.UMJ2023_Scroll")
          (set `self.AdditionValue` 3.0)
          (set `self.SubtractValue` 0.0))
        (:`NewEnumerator4`
          (set `self.SetMesh` "/Game/ASSETS/UMJ2023_Book.UMJ2023_Book")
          (set `self.AdditionValue` 6.0)
          (set `self.SubtractValue` 0.0))
        (:`NewEnumerator1`
          (set `self.SetMesh` "/Game/ASSETS/UMJ2023_Cassette.UMJ2023_Cassette")
          (set `self.AdditionValue` 8.0)
          (set `self.SubtractValue` 0.0))
        (:`NewEnumerator2`
          (set `self.SetMesh` "/Game/ASSETS/UMJ2023_Floppy.UMJ2023_Floppy")
          (set `self.AdditionValue` 10.0)
          (set `self.SubtractValue` 0.0))
        (:`NewEnumerator3`
          (set `self.SetMesh` "/Game/ASSETS/UMJ2023_CD.UMJ2023_CD")
          (set `self.AdditionValue` 12.0)
          (set `self.SubtractValue` 0.0))
        (:`NewEnumerator5`
          (set `self.SetMesh` "/Game/ASSETS/UMJ2023_USB.UMJ2023_USB")
          (set `self.AdditionValue` 15.0)
          (set `self.SubtractValue` 0.0))
        (:`NewEnumerator6`
          (set `self.SetMesh` "/Game/ASSETS/UMJ2023_HDD.UMJ2023_HDD")
          (set `self.AdditionValue` 20.0)
          (set `self.SubtractValue` 0.0))
        (:`NewEnumerator7`
          (set `self.SetMesh` "/Game/ASSETS/UMJ2023_SSD.UMJ2023_SSD")
          (set `self.AdditionValue` 25.0)
          (set `self.SubtractValue` 0.0)))
      (`StaticMeshComponent.SetStaticMesh` (`self.StaticMesh`) (`self.SetMesh`))
      (`PrimitiveComponent.SetCollisionEnabled` (`self.StaticMesh`) "NoCollision"))))

(event `/Game/BLUEPRINTS/BPI_Interface.TokenDrop`
  ;[0.05729 0.05729 0.05729] Drop item at player's location on that tick / Attach item to player
  (`self.CheckForPlatform`)
  (message `/Game/BLUEPRINTS/BPI_Interface.SetPlatformHeight` (`self.PlatformRef`) (`self.AdditionValue`) self)
  (`PrimitiveComponent.SetCollisionEnabled` (`self.Box`) "QueryAndPhysics"))

(event `self.ReceiveTick`
  (params (DeltaSeconds :type "Float (single-precision)")))

(event `/Game/BLUEPRINTS/BPI_Interface.TokenPickup`
  ;[0.05729 0.05729 0.05729] Drop item at player's location on that tick / Attach item to player
  (message `/Game/BLUEPRINTS/BPI_Interface.SetPlatformHeight` (`self.PlatformRef`) (* (`self.AdditionValue`) -1.0) self)
  (`PrimitiveComponent.SetCollisionEnabled` (`self.Box`) "NoCollision"))

(fn `CheckForPlatform`
  (bind _returnvalue (`self.K2_GetActorLocation`))
  (bind _outhit (`KismetSystemLibrary.SphereTraceSingleForObjects` :`Start` _returnvalue :`End` (- _returnvalue (0.0 0.0 100.0)) :`Radius` 50.0 :`ObjectTypes` (`|MakeArray` "ObjectTypeQuery1" :!type "EObjectTypeQuery Enum") :`DrawDebugType` "ForDuration"))
  (if (`self.ActorHasTag` (`.HitActor` (`GameplayStatics.BreakHitResult` _outhit)) "Platform")
    (set `self.PlatformRef` (`.HitActor` (`GameplayStatics.BreakHitResult` _outhit)))
    (return)))

(fn `UserConstructionScript`)