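; BP_VictoryVolume is a trigger volume that ends play with a win screen when the player reaches it.
; Its collision overlap checks for the "Player" tag, casts to BP_Player and destroys that actor.
; It then adds a win screen widget to the viewport, shows the mouse cursor and removes top-level UI widgets from the screen.
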(event `self.Collision.OnComponentBeginOverlap`
  (params (OverlappedComponent :type "PrimitiveComponent Object Reference") (OtherActor :type "Actor Object Reference") (OtherComp :type "PrimitiveComponent Object Reference") (OtherBodyIndex :type Integer) (bFromSweep :type Boolean) (SweepResult :type "HitResult Structure (by ref)"))
  (if (`self.ActorHasTag` OtherActor "Player")
    (bind _asbp_player (cast `/Game/CHARACTERS/PlayerChar/BP_Player` OtherActor))
    (`self.K2_DestroyActor` _asbp_player)
    (`|ExecutionSequence`
      (:`then_0`
        (bind _returnvalue (`|CreateWidget` "/Game/BLUEPRINTS/WIDGETS/WinScreen.WinScreen_C"))
        (`UserWidget.AddToViewport` _returnvalue 0)
        (set `PlayerController.bShowMouseCursor` true (`GameplayStatics.GetPlayerController` 0)))
      (:`then_1`
        (bind _foundwidgets (`WidgetBlueprintLibrary.GetAllWidgetsOfClass` "/Game/BLUEPRINTS/WIDGETS/UI.UI_C"))
        (`Widget.RemoveFromParent` _foundwidgets)))))

(fn `UserConstructionScript`)