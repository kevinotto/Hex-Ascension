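; Enemy spawner actor that periodically spawns a BP_Enemy at a random spawn point.
; The construction script gathers seven spawn point components into an array.
; BeginPlay slows the actor's tick interval so Tick acts as the spawn timer, with no cap on enemy count.
; The random index range runs one past the array's last element, so some picks fall outside it.
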(event `self.ReceiveBeginPlay`
  (`self.SetActorTickInterval` 5.0))

(event `self.ReceiveTick`
  (params (DeltaSeconds :type "Float (single-precision)"))
  (`|SpawnActorFromClass` "/Game/BLUEPRINTS/BP_Enemy.BP_Enemy_C" (`KismetMathLibrary.MakeTransform` (`SceneComponent.K2_GetComponentLocation` (`|GetArrayItem` (`self.SpawnsArray`) (`KismetMathLibrary.RandomIntegerInRange` 0 7)))) "Undefined" "MultiplyWithRoot" null null))

(fn `UserConstructionScript`
  (set `self.SpawnsArray` (`|MakeArray` (`self.Spawnpoint`) (`self.Spawnpoint1`) (`self.Spawnpoint2`) (`self.Spawnpoint3`) (`self.Spawnpoint4`) (`self.Spawnpoint5`) (`self.Spawnpoint6`))))