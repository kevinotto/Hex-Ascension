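; BP_Enemy is an enemy that homes in on the player, damages them on proximity and drops a BP_Token when hit.
; BeginPlay sets the player's mesh as the ProjectileMovement homing target and disables capsule physics if vertical velocity is zero.
; Tick uses a Delay to run a sphere trace about every half second, damaging a hit Pawn tagged Player.
; Any damage destroys it; an older interpolation-based follow chain is left unconnected.
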(event `self.ReceiveAnyDamage`
  (params (Damage :type "Float (single-precision)") (DamageType :type "DamageType Object Reference") (InstigatedBy :type "Controller Object Reference") (DamageCauser :type "Actor Object Reference"))
  ;[1 1 1] Enemy death from player's hit and tokenb spawn on ssame place
  (`self.K2_DestroyActor`)
  (`|SpawnActorFromClass` "/Game/BLUEPRINTS/BP_Token.BP_Token_C" (`KismetMathLibrary.MakeTransform` (`self.K2_GetActorLocation`)) "Undefined" "MultiplyWithRoot" null null))

(event `self.ReceiveTick`
  (params (DeltaSeconds :type "Float (single-precision)"))
  (bind _returnvalue (`self.K2_GetActorLocation`))
  ;[1 1 1] Follows player
  (`KismetSystemLibrary.Delay` 0.5)
  (bind _outhit (`KismetSystemLibrary.SphereTraceSingleForObjects` _returnvalue _returnvalue 75.0 (`|MakeArray` "ObjectTypeQuery3" :!type "EObjectTypeQuery Enum") false (`|MakeArray` self :!type "Actor Object Reference") "ForOneFrame"))
  (if (`self.ActorHasTag` (`.HitActor` (`GameplayStatics.BreakHitResult` _outhit)) "Player")
    (`GameplayStatics.ApplyDamage` (`.HitActor` (`GameplayStatics.BreakHitResult` _outhit)) 1.0)))

(event `self.ReceiveBeginPlay`
  (bind (_velocity_x _velocity_y _velocity_z) (`KismetMathLibrary.BreakVector` (`MovementComponent.Velocity` (`self.CharacterMovement`))))
  (bind _asbp_player (cast `/Game/CHARACTERS/PlayerChar/BP_Player` (`GameplayStatics.GetPlayerCharacter` 0)))
  (set `ProjectileMovementComponent.HomingTargetComponent` (`Character.Mesh` _asbp_player) (`self.ProjectileMovement`))
  (if (== _velocity_z 0.0)
    (`PrimitiveComponent.SetSimulatePhysics` (`self.CapsuleComponent`) false)))

(fn `UserConstructionScript`)